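; Skybox actor that applies a chosen material to its static mesh and exposes sky look settings as editable variables.
; Its construction script pushes power, star brightness, scene brightness and RGB color values into the SkyBoxParam material parameter collection.
; All work happens at construction; the event graph holds only disabled stub events, so nothing updates at runtime.
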(event EventBeginPlay)

(event Collision|EventActorBeginOverlap
  (params (OtherActor :type Actor%20Object%20Reference)))

(event EventTick
  (params (DeltaSeconds :type Float%20%28single-precision%29)))

(fn ConstructionScript
  (Rendering|Material|SetMaterial (Variables|Default|GetStaticMesh) 0 (Variables|Default|GetMaterial))
  (Rendering|Material|SetScalarParameterValue "/Game/Materials/SkyBoxParam.SkyBoxParam" "Power" (Variables|Default|GetPower) :!class /Script/Engine.KismetMaterialLibrary)
  (Rendering|Material|SetScalarParameterValue "/Game/Materials/SkyBoxParam.SkyBoxParam" "Star Brightness" (Variables|Default|GetStar%20Brightness) :!class /Script/Engine.KismetMaterialLibrary)
  (Rendering|Material|SetScalarParameterValue "/Game/Materials/SkyBoxParam.SkyBoxParam" "Scene Brightness" (Variables|Default|GetScene%20Brightness) :!class /Script/Engine.KismetMaterialLibrary)
  (Rendering|Material|SetScalarParameterValue "/Game/Materials/SkyBoxParam.SkyBoxParam" "Red" (Variables|Default|GetRed) :!class /Script/Engine.KismetMaterialLibrary)
  (Rendering|Material|SetScalarParameterValue "/Game/Materials/SkyBoxParam.SkyBoxParam" "Green" (Variables|Default|GetGreen) :!class /Script/Engine.KismetMaterialLibrary)
  (Rendering|Material|SetScalarParameterValue "/Game/Materials/SkyBoxParam.SkyBoxParam" "Blue" (Variables|Default|GetBlue) :!class /Script/Engine.KismetMaterialLibrary))